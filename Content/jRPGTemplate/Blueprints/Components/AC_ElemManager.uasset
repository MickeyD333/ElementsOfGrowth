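; Actor component from a jRPG template that manages an inventory of Elems stored in the game instance.
; AddElemToInventory looks up the Elem's row in DT_jRPG_Elements by hardcoded name, then calls CheckIfElemIsInInventory.
; That check loops the Elems array until the name matches and returns success, index and whether the stack is at its maximum.
; The add logic is unfinished: it stops after the stack-full check and never changes the inventory.
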(event EventBeginPlay)

(event EventTick
  (params (DeltaSeconds :type Float%20%28single-precision%29)))

(fn AddElemtoInventory
  (params (ElemHardcodedName :type Name) (Amount :type Integer))
  (LocalVariables|SetElemHardcodedName%20LOCAL ElemHardcodedName) ; Setting input to local variable
  (LocalVariables|SetAmountToAdd%20LOCAL Amount) ; Setting input to local variable
  (bind _returnvalue (Utilities|GetDataTableRow "/Game/jRPGTemplate/Datatables/DT_jRPG_Elements.DT_jRPG_Elements" (LocalVariables|GetElemHardcodedName%20LOCAL)) ; Getting data of Elem
    (:then
      (LocalVariables|SetElemStructLocal _returnvalue) ; Setting data of Elem to local variable
      (bind (_success_ _iselemfullystacked_ _elemindex) (CallFunction|CheckifElemIsinInventory (LocalVariables|GetElemHardcodedName%20LOCAL)))
      (if _success_ ; If we succeeded in finding the Elem in our inventory...
        (if (not _iselemfullystacked_) ; ...then we check to make sure the stack isn't full.
          _)))))

(fn CheckifElemIsinInventory
  (params (ElemHardcodedName :type Name))
  (bind (_array_element _array_index) (Utilities|Array|ForEachLoopwithBreak (Variables|/Game/jRPGTemplate/Blueprints/Basics/BP_jRPG_GI_Custom.BP_jRPG_GI_Custom_C|GetElems (Variables|Default|GetGame%20Instance%20Reference)) :!label _label) ; Loop through array given and stop at end.
    (:LoopBody
      (if (== (.ElemHardcodedName (Utilities|Struct|BreakS_jRPG_Elements_StaticData (.ElemStaticData (Utilities|Struct|BreakS_jRPG_Elements_DynamicData _array_element)))) ElemHardcodedName) ; ...we continue on...
        (LocalVariables|SetSuccess?LOCAL true) ; ..to set success as true.
        (LocalVariables|SetIsElemFullyStacked?LOCAL (== (.StacksAmount (Utilities|Struct|BreakS_jRPG_Elements_DynamicData _array_element)) (.ElemMaxStackAmount (Utilities|Struct|BreakS_jRPG_Elements_StaticData (.ElemStaticData (Utilities|Struct|BreakS_jRPG_Elements_DynamicData _array_element)))))) ; ...we declare the fully stacked variable true.
        (LocalVariables|SetElemIndexLOCAL _array_index) ; Setting local variable to Elem we're at in the list. If it's not right, loop back through.
        (goto _label Break)))
    (:Completed
      (return (LocalVariables|GetSuccess?LOCAL) (LocalVariables|GetIsElemFullyStacked?LOCAL) (LocalVariables|GetElemIndexLOCAL)) ; Returning values
    )))